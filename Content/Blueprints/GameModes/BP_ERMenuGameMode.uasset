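; BP_ERMenuGameMode is the game mode for the main menu, setting up the front-end UI when play begins.
; BeginPlay creates and displays the start menu widget, plus an options widget that starts collapsed, keeping references to both.
; It also switches the player to UI-only input with a visible cursor, reloads saved game user settings and plays an ambient music track.
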(event `self.ReceiveBeginPlay`
  (`|ExecutionSequence`
    (:`then_0`
      (bind _returnvalue (`|CreateWidget` "/Game/Blueprints/Menu/StartMenu/WBP_ERStartMenu.WBP_ERStartMenu_C"))
      (bind _output_get (set `self.StartMenuRef` _returnvalue))
      (`UserWidget.AddToViewport` _output_get 0))
    (:`then_1`
      (bind _returnvalue_2 (`|CreateWidget` "/Game/Blueprints/Menu/Options/WBP_ERMenuOptions.WBP_ERMenuOptions_C"))
      (bind _output_get_2 (set `self.MenuOptionsRef` _returnvalue_2))
      (`UserWidget.AddToViewport` _output_get_2 0)
      (`Widget.SetVisibility` (`self.MenuOptionsRef`) "Collapsed"))
    (:`then_2`
      (`WidgetBlueprintLibrary.SetInputMode_UIOnlyEx` (`GameplayStatics.GetPlayerController` 0) null)
      (set `PlayerController.bShowMouseCursor` true (`GameplayStatics.GetPlayerController` 0)))
    (:`then_3`
      (bind _returnvalue_3 (`GameUserSettings.GetGameUserSettings`))
      (`GameUserSettings.LoadSettings` _returnvalue_3 true))
    (:`then_4`
      (`GameplayStatics.PlaySound2D` "/Game/Audio/Music/apathias-dark-ambient-sad-music-277034.apathias-dark-ambient-sad-music-277034" 1.0 1.0 0.0 null null))))

(fn `UserConstructionScript`)