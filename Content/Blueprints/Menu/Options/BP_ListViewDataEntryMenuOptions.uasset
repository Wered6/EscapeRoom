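; Data object for one row in the options menu list view, representing a setting shown as either a check box or a drop-down.
; Init takes the row's widgets, sets the label, activates the control matching SelectionMode and fills the drop-down, selecting its first option.
; It binds the control's change event, re-broadcasts changes through its own dispatchers, and returns the description text and switcher.
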(fn `Init`
  (params (WidgetSwitcherSelectMode :type "WidgetSwitcher Object Reference") (CheckBox :type "CheckBox Object Reference") (DropDownBox :type "ComboBoxString Object Reference") (Text :type "TextBlock Object Reference") (MenuOptionsListViewRef :type "/Game/Blueprints/Menu/Options/WBP_MenuOptionsListView Object Reference"))
  (returns (DescText :type Text) (WidgetSwitcherDesc :type "WidgetSwitcher Object Reference"))
  (bind _dropdownoptions (`self.DropDownOptions`))
  (set `self.MenuOptionsListViewRef` MenuOptionsListViewRef)
  (`TextBlock.SetText` (`local.Text`) (`self.Text`))
  (switch `/Game/Blueprints/Menu/Options/ESelectionMode` (`self.SelectionMode`)
    (:`NewEnumerator0`
      (`WidgetSwitcher.SetActiveWidget` (`local.WidgetSwitcherSelectMode`) (`local.CheckBox`))
      (add `CheckBox.OnCheckStateChanged` (`local.CheckBox`) (`|CreateDelegate` :!event `OnCheckStateChangedFunc`))
      (return (`self.DescText`) (`self.WidgetSwitcherDesc`)))
    (:`NewEnumerator1`
      (`WidgetSwitcher.SetActiveWidget` (`local.WidgetSwitcherSelectMode`) (`local.DropDownBox`))
      (for _array_element (`self.DropDownOptions`)
        (`ComboBoxString.AddOption` (`local.DropDownBox`) _array_element))
      (if (`KismetArrayLibrary.Array_IsValidIndex` _dropdownoptions)
        (`ComboBoxString.SetSelectedOption` (`local.DropDownBox`) (`|GetArrayItem` _dropdownoptions))
        (add `ComboBoxString.OnSelectionChanged` (`local.DropDownBox`) (`|CreateDelegate` :!event `OnSelectionChangedFunc`))
        (return (`self.DescText`) (`self.WidgetSwitcherDesc`))))))

(fn `OnCheckStateChangedFunc`
  (params (bIsChecked :type Boolean))
  (`self.OnCheckStateChanged` bIsChecked))

(fn `OnSelectionChangedFunc`
  (params (SelectedItem :type String) (SelectionType :type "ESelectInfo Enum" :default "OnKeyPress"))
  (`self.OnSelectionChanged` SelectedItem SelectionType))