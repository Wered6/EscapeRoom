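; BP_CabinetDrawerBase is an interactable cabinet drawer that can be locked.
; On interaction it calls the parent handler, then checks its LockComponent.
; A locked drawer plays a short timeline that nudges the mesh along local Y as a failed pull attempt.
; An unlocked drawer uses a FlipFlop to play or reverse a timeline that slides it open and closed by a pull distance.
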(event `ERInteractInterface.InteractStart`
  (params (OtherInstigator :type "Actor Object Reference"))
  (`parent.InteractStart` OtherInstigator)
  (if (`ERLockComponent.GetIsLocked` (`self.LockComponent`))
    (bind (_direction _drawertrymove) (`Timeline|TryOpenDrawerTimeline` :!via `PlayFromStart`)
      (:`Update`
        (`SceneComponent.K2_SetRelativeLocation` (`self.RootMesh`) (`KismetMathLibrary.MakeVector` 0.0 (* _drawertrymove (`self.DrawerTryMoveStr`))) false false)))
    (else
      (`/Engine/EditorBlueprintResources/StandardMacros.FlipFlop`
        (:`A`
          (bind (_direction_2 _drawermovement) (`Timeline|OpenDrawerTimeline` :!label _label)
            (:`Update`
              (`SceneComponent.K2_SetRelativeLocation` (`self.RootMesh`) (`KismetMathLibrary.MakeVector` 0.0 (* _drawermovement (`self.DrawerPullDist`))) false false))))
        (:`B`
          (goto _label :!via `Reverse`))))))

(fn `UserConstructionScript`)