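; Base Blueprint for an interactable cabinet door that swings open and closed, or rattles when locked.
; InteractStart runs the parent logic, then checks Locked.
; A locked door plays a short try-open timeline, while an unlocked one alternates a timeline forward and in reverse through a FlipFlop.
; Both timelines drive scaled RootMesh yaw, and finishing the open/close timeline sets InteractArea's collision profile to "InteractArea".
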(event `ERInteractInterface.InteractStart`
  (params (OtherInstigator :type "Actor Object Reference"))
  (`parent.InteractStart` OtherInstigator)
  (if (`self.bLocked`)
    (bind (_direction _doortryrotate) (`Timeline|TryOpenDoorTimeline` :!via `PlayFromStart`)
      (:`Update`
        (`SceneComponent.K2_SetRelativeRotation` (`self.RootMesh`) (`KismetMathLibrary.MakeRotator` 0.0 0.0 (* _doortryrotate (`self.DoorTryRotateStr`))) false false)))
    (else
      (`/Engine/EditorBlueprintResources/StandardMacros.FlipFlop`
        (:`A`
          (bind (_direction_2 _doorrotation) (`Timeline|OpenDoorTimeline` :!label _label)
            (:`Update`
              (`SceneComponent.K2_SetRelativeRotation` (`self.RootMesh`) (`KismetMathLibrary.MakeRotator` 0.0 0.0 (* _doorrotation (`self.DoorRotationAngle`))) false false))
            (:`Finished`
              (`PrimitiveComponent.SetCollisionProfileName` (`self.InteractArea`) "InteractArea" true))))
        (:`B`
          (goto _label :!via `Reverse`))))))

(fn `UserConstructionScript`)