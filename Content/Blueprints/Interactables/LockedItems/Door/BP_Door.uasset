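; BP_Door is an interactable door that either swings open or rattles, depending on whether its lock component reports locked.
; On InteractStart it runs the parent logic, then restarts a try-open timeline if locked or plays the open timeline otherwise.
; Both timelines drive door yaw and handle roll, scaled by angle and strength variables.
; The graph has no closing path.
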(event `ERInteractInterface.InteractStart`
  (params (OtherInstigator :type "Actor Object Reference"))
  (`parent.InteractStart` OtherInstigator)
  (if (`ERLockComponent.GetIsLocked` (`self.LockComponent`))
    (bind (_direction _doortryrotate _handlerotation) (`Timeline|TryOpenDoorTimeline` :!via `PlayFromStart`)
      (:`Update`
        (`SceneComponent.K2_SetRelativeRotation` (`self.DoorMesh`) (`KismetMathLibrary.MakeRotator` 0.0 0.0 (* _doortryrotate (`self.DoorTryRotateStr`) -1.0)) false false)
        (`SceneComponent.K2_SetRelativeRotation` (`self.HandleMesh`) (`KismetMathLibrary.MakeRotator` (* _handlerotation (`self.HandleRotationAngle`) -1.0)) false false)))
    (else
      (bind (_direction_2 _doorrotation _handlerotation_2) (`Timeline|OpenDoorTimeline`)
        (:`Update`
          (`SceneComponent.K2_SetRelativeRotation` (`self.DoorMesh`) (`KismetMathLibrary.MakeRotator` 0.0 0.0 (* _doorrotation (`self.DoorRotationAngle`) -1.0)) false false)
          (`SceneComponent.K2_SetRelativeRotation` (`self.HandleMesh`) (`KismetMathLibrary.MakeRotator` (* _handlerotation_2 (`self.HandleRotationAngle`) -1.0)) false false))))))

(fn `UserConstructionScript`)