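; BP_LampSwitch is an interactable wall or prop switch that toggles a referenced Lamp.
; Each press blocks further interaction, and a FlipFlop alternately plays or reverses a Timeline that rolls the switch mesh by a scaled angle.
; When the Timeline finishes, interaction is re-enabled and TurnLights is called on the Lamp, or a debug message prints if that reference is invalid.
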(event `self.InteractPressTriggered`
  (`parent.InteractPressTriggered`)
  (`self.SetCanInteract` false)
  (`/Engine/EditorBlueprintResources/StandardMacros.FlipFlop`
    (:`A`
      (bind (_direction _switchrotation) (`Timeline|Timeline` :!label _label)
        (:`Update`
          (`SceneComponent.K2_SetRelativeRotation` (`self.SwitchMesh`) (`KismetMathLibrary.MakeRotator` (* (* _switchrotation (`self.SwitchRotationAngle`)) -1.0)) false false))
        (:`Finished`
          (`self.SetCanInteract` true)
          (bind _lamp (`self.Lamp`)
            (:`then`
              (`ERCeilingLamp.TurnLights` _lamp))
            (:`else`
              (`KismetSystemLibrary.PrintString` "BP_LampSwitch, Lamp is nullptr"))))))
    (:`B`
      (goto _label :!via `Reverse`))))

(fn `UserConstructionScript`)