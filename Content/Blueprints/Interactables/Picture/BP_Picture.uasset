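; BP_Picture is an interactable picture that swings on its yaw axis when the player presses interact.
; Each press alternates through a FlipFlop between playing and reversing a timeline, whose curve, scaled by PictureRotationAngle, drives the relative rotation of the painting and back meshes.
; On BeginPlay it registers both meshes as outline components with InteractableComp, and it exposes WidgetAttachment as the widget attachment component.
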(event `self.ReceiveBeginPlay`
  (`ERInteractableComponent.SetOutlineMeshComponents` (`self.InteractableComp`) (`|MakeArray` (`self.PaintingMesh`) (`self.BackMesh`) :!type "MeshComponent Object Reference")))

(event `ERInteractInterface.InteractPressTriggered`
  (`parent.InteractPressTriggered`)
  (`/Engine/EditorBlueprintResources/StandardMacros.FlipFlop`
    (:`A`
      (bind (_direction _picturerotation) (`Timeline|Timeline` :!label _label)
        (:`Update`
          (`SceneComponent.K2_SetRelativeRotation` (`self.PaintingMesh`) (`KismetMathLibrary.MakeRotator` 0.0 0.0 (* _picturerotation (`self.PictureRotationAngle`))) false false)
          (`SceneComponent.K2_SetRelativeRotation` (`self.BackMesh`) (`KismetMathLibrary.MakeRotator` 0.0 0.0 (* _picturerotation (`self.PictureRotationAngle`))) false false))))
    (:`B`
      (goto _label :!via `Reverse`))))

(fn `GetWidgetAttachmentComponent`
  (returns (ReturnValue :type "SceneComponent Object Reference"))
  (return (`self.WidgetAttachment`)))

(fn `UserConstructionScript`)